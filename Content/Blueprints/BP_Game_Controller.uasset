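; BP_Game_Controller is a player-side controller that sets up HUD widgets, interaction timers and input-device tracking.
; Initialize caches the character's capsule size, starts looping name-based timers for interaction tracing and nearby-object highlighting, then creates subtitle and message widgets.
; InitializeInput and UpdateInputDevice sync the gamepad flag with user settings and broadcast it to all widgets.
; DisplayMessage forwards notifications to the message widget; CloseGameMenu is an empty stub.
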(fn `CloseGameMenu`)

(fn `DisplayMessage`
  (params (`Message Text` :type Text))
  (`/Game/UI/W_Message_Hud.Show Notification` (`self.MessageWidget`) `Message Text`))

(fn `Initialize`
  (bind _ascharacter (cast `Character` (`GameplayStatics.GetPlayerPawn` 0)))
  (bind _capsulecomponent (`Character.CapsuleComponent` _ascharacter))
  (set `self.PlayerCapsuleRadius` (`CapsuleComponent.GetScaledCapsuleRadius` _capsulecomponent))
  (set `self.PlayerCapsuleHalfHeight` (`CapsuleComponent.GetScaledCapsuleHalfHeight` _capsulecomponent))
  (`KismetSystemLibrary.K2_SetTimer` null "TraceForInteraction" 0.0 true)
  (`KismetSystemLibrary.K2_SetTimer` null "FindAndHighlightObjectsNearPlayer" 0.1 true)
  (bind _returnvalue (`|CreateWidget` "/Game/UI/W_Subtitles.W_Subtitles_C"))
  (bind _output_get (set `self.SubtitlesWidget` _returnvalue))
  (`UserWidget.AddToViewport` _output_get 1)
  (bind _returnvalue_2 (`|CreateWidget` "/Game/UI/W_Message_Hud.W_Message_Hud_C"))
  (bind _output_get_2 (set `self.MessageWidget` _returnvalue_2))
  (`UserWidget.AddToViewport` _output_get_2 10)
  (`self.InitializeInput`))

(fn `InitializeInput`
  (set `self.GamepadInput` (`/Game/Blueprints/Save/BP_User_Settings.GamepadInput` (`/Game/Blueprints/BP_Game_Instance.Get User Settings` (`/Game/Blueprints/Classes/BP_Function_Library.GetGameInstance`))))
  (bind _foundwidgets (`WidgetBlueprintLibrary.GetAllWidgetsOfClass` "/Script/UMG.UserWidget" false))
  (for _array_element _foundwidgets
    (message `/Game/Blueprints/BP_WidgetInterface.ControlMethodChanged` _array_element (`self.GamepadInput`))))

(fn `UpdateInputDevice`
  (params (Key :type "Key Structure (by ref)"))
  (bind _returnvalue (`KismetInputLibrary.Key_IsGamepadKey` Key))
  (if (!= (`self.GamepadInput`) _returnvalue)
    (bind _output_get (set `self.GamepadInput` _returnvalue))
    (set `/Game/Blueprints/Save/BP_User_Settings.GamepadInput` _output_get (`/Game/Blueprints/BP_Game_Instance.Get User Settings` (`/Game/Blueprints/Classes/BP_Function_Library.GetGameInstance`)))
    (bind _foundwidgets (`WidgetBlueprintLibrary.GetAllWidgetsOfClass` "/Script/UMG.UserWidget" false))
    (for _array_element _foundwidgets
      (message `/Game/Blueprints/BP_WidgetInterface.ControlMethodChanged` _array_element (`self.GamepadInput`)))))

(fn `UserConstructionScript`)