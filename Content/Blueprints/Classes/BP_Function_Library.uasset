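; Blueprint function library with shared getters for the game's controller, instance and mode, plus a widget visibility helper.
; GetGameController returns the first BP_Game_Controller actor found, while the instance and mode getters return casts to their BP classes.
; HideActiveWidgets gathers visible top-level widgets, excluding two classes, and returns them.
; Despite its name, it sets their visibility to Visible rather than a hidden state.
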(fn `GetGameController`
  (returns (GameController :type "/Game/Blueprints/BP_Game_Controller Object Reference"))
  (bind _outactors (`GameplayStatics.GetAllActorsOfClass` null "/Game/Blueprints/BP_Game_Controller.BP_Game_Controller_C"))
  (return (`|GetArrayItem` _outactors)))

(fn `GetGameInstance`
  (returns (`Game Instance` :type "/Game/Blueprints/BP_Game_Instance Object Reference"))
  (bind _asbp_game_instance (cast `/Game/Blueprints/BP_Game_Instance` (`GameplayStatics.GetGameInstance` null)))
  (return _asbp_game_instance))

(fn `GetGameMode`
  (returns (`Game Mode` :type "/Game/Blueprints/BP_Game_Mode Object Reference"))
  (bind _asbp_game_mode (cast `/Game/Blueprints/BP_Game_Mode` (`GameplayStatics.GetGameMode` null)))
  (return _asbp_game_mode))

(fn `HideActiveWidgets`
  (returns (HiddenWidgets :type "Array of UserWidget Object Reference"))
  (locals (Widgets :type "Array of UserWidget Object Reference"))
  (bind _foundwidgets (`WidgetBlueprintLibrary.GetAllWidgetsOfClass` (`local.__WorldContext`) "/Script/UMG.UserWidget"))
  (for _array_element _foundwidgets
    (bind _returnvalue (`GameplayStatics.GetObjectClass` _array_element))
    (if (and (`Widget.IsVisible` _array_element) (!= _returnvalue null) (!= _returnvalue null))
      (`Widget.SetVisibility` _array_element "Visible")
      (`KismetArrayLibrary.Array_Add` (`local.Widgets`) _array_element)))
  (return (`local.Widgets`)))